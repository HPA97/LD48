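; Player controller for a depth-scoring game, handling HUD widgets, high score persistence and restart or quit keys.
; On begin play it loads the high score, shows a score widget and briefly displays a tip, while Tick records the character's Z as current depth.
; Setting the depth score hides the score widget, saves any lower Z as the new record to the HS save slot, then opens the menu.
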(event Custom|Set_Depth_Score
  (Widget|SetVisibility (Variables|Default|GetScore) "Collapsed")
  (Variables|Default|SetDepth_Score (Variables|Default|GetCurrent_Depth))
  (Utilities|FlowControl|Sequence
    (:then_0
      (if (< (Variables|Default|GetDepth_Score) (Variables|Default|GetHighScore))
        (Variables|Default|SetHighScore (Variables|Default|GetDepth_Score))
        (CallFunction|SaveHighscore)))
    (:then_1
      (bind _returnvalue (UserInterface|CreateWidget "/Game/Widgets/Menu.Menu_C"))
      (UserInterface|Viewport|AddtoViewport _returnvalue 0))))

(event Custom|Load_Highscore
  (bind _returnvalue (SaveGame|DoesSaveGameExist "HS"))
  (if _returnvalue
    (bind _returnvalue_2 (SaveGame|LoadGamefromSlot "HS"))
    (bind _ashs_sg (Utilities|Casting|CastToHS_SG _returnvalue_2))
    (Variables|Default|SetHighScore (Variables|/Game/Blueprints/HS_SG.HS_SG_C|GetHighScore _ashs_sg))
    (else
      (bind _returnvalue_3 (SaveGame|CreateSaveGameObject "/Game/Blueprints/HS_SG.HS_SG_C"))
      (bind _ashs_sg_2 (Utilities|Casting|CastToHS_SG _returnvalue_3))
      (Variables|/Game/Blueprints/HS_SG.HS_SG_C|SetHighScore _ashs_sg_2 (Variables|Default|GetHighScore))
      (SaveGame|SaveGametoSlot _ashs_sg_2 "HS"))))

(event Custom|Save_highscore
  (bind _returnvalue (SaveGame|DoesSaveGameExist "HS"))
  (if _returnvalue
    (bind _returnvalue_2 (SaveGame|LoadGamefromSlot "HS"))
    (bind _ashs_sg (Utilities|Casting|CastToHS_SG _returnvalue_2))
    (Variables|/Game/Blueprints/HS_SG.HS_SG_C|SetHighScore _ashs_sg (Variables|Default|GetHighScore))
    (SaveGame|SaveGametoSlot _ashs_sg "HS")
    (else
      (bind _returnvalue_3 (SaveGame|CreateSaveGameObject "/Game/Blueprints/HS_SG.HS_SG_C"))
      (bind _ashs_sg_2 (Utilities|Casting|CastToHS_SG _returnvalue_3))
      (Variables|/Game/Blueprints/HS_SG.HS_SG_C|SetHighScore _ashs_sg_2 (Variables|Default|GetHighScore))
      (SaveGame|SaveGametoSlot _ashs_sg_2 "HS"))))

(event EventBeginPlay
  (bind _returnvalue (UserInterface|CreateWidget "/Game/Widgets/Tip.Tip_C"))
  (UserInterface|Viewport|AddtoViewport _returnvalue 0)
  (Variables|Default|SetTip _returnvalue)
  (CallFunction|LoadHighscore)
  (Utilities|FlowControl|Delay 0.2)
  (Variables|Default|SetPlayer_Character (Game|GetPlayerCharacter 0))
  (bind _returnvalue_2 (UserInterface|CreateWidget "/Game/Widgets/Score.Score_C"))
  (UserInterface|Viewport|AddtoViewport _returnvalue_2 0)
  (Variables|Default|SetScore _returnvalue_2)
  (Utilities|FlowControl|Delay 5.0)
  (Widget|SetVisibility (Variables|Default|GetTip) "Collapsed"))

(event EventTick
  (params (DeltaSeconds :type Float%20%28single-precision%29))
  (bind _returnvalue (Game|GetPlayerCharacter 0))
  (if (Utilities|IsValid _returnvalue)
    (Variables|Default|SetCurrent_Depth (.Z (Math|Vector|BreakVector (Transformation|GetActorLocation _returnvalue))))))

(event Input|KeyboardEvents|R
  (params (Key :type Key%20Structure :default "None"))
  (:Pressed
    (Game|OpenLevel(byName) "Main_M")))

(event Input|KeyboardEvents|Escape
  (params (Key :type Key%20Structure :default "None"))
  (:Pressed
    (Game|QuitGame 0 "Quit" false)))

(fn ConstructionScript)