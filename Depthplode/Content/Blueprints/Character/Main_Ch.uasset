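; Player character that moves along a single horizontal axis, jumps with a sound, and shows a left, middle or right eye to match input direction.
; Destroy has Main_PC set the depth score, moves the character to a fixed X/Y at its current height, and alters its acceleration, gravity and point light.
; It also plays a fail sound through a spawned Sound_Object, as jumping does, then destroys the actor after a long delay.
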(event Custom|Destroy
  (bind _charactermovement (Variables|Character|GetCharacterMovement))
  (bind _pointlight (Variables|Default|GetPointLight))
  (bind _pointlight_2 (Variables|Default|GetPointLight))
  (bind _returnvalue (Transformation|GetRelativeTransform _pointlight))
  (bind _location (Math|Transform|BreakTransform _returnvalue))
  (bind (_x _y _z) (Math|Vector|BreakVector _location))
  (bind _asmain_pc (Utilities|Casting|CastToMain_PC (Game|GetPlayerController 0)))
  (Default|SetDepthScore _asmain_pc)
  (Utilities|FlowControl|Sequence
    (:then_0
      (Transformation|SetActorLocation (Math|Vector|MakeVector 3.5e+03 3.4e+02 (.Z (Math|Vector|BreakVector (Transformation|GetActorLocation)))) false false)
      (Rendering|Lighting|SetAttenuationRadius _pointlight_2 9e+03)
      (Variables|/Script/Engine.CharacterMovementComponent|SetMaxAcceleration _charactermovement 5e+02)
      (Variables|/Script/Engine.CharacterMovementComponent|SetGravityScale _charactermovement 1.0)
      (bind _returnvalue_2 (Game|SpawnActorfromClass "/Game/Sounds/Sound_Object.Sound_Object_C" (Math|Transform|MakeTransform (Transformation|GetActorLocation)) "Undefined" 0 0))
      (Default|PlaySound _returnvalue_2 "/Game/Sounds/fail_01.fail_01")
      (Rendering|SetVisibility _pointlight_2 true false)
      (Rendering|Components|Light|SetIntensity (Variables|Default|GetPointLight) 1e+04)
      (Transformation|SetRelativeLocation (Variables|Default|GetPointLight) (Math|Vector|MakeVector (+ _x 2.5e+02) _y _z) false false))
    (:then_1
      (Utilities|FlowControl|Delay 5e+01)
      (Actor|DestroyActor))))

(event Input|ActionEvents|InputActionJump
  (params (Key :type Key%20Structure :default "None"))
  (:Pressed
    (Character|Jump)
    (bind _returnvalue (Game|SpawnActorfromClass "/Game/Sounds/Sound_Object.Sound_Object_C" (Math|Transform|MakeTransform (Transformation|GetActorLocation)) "Undefined" 0 0))
    (Default|PlaySound _returnvalue "/Game/Sounds/jump_01.jump_01"))
  (:Released
    (Character|StopJumping)))

(event Input|AxisEvents|InputAxisMoveRight
  (params (AxisValue :type Float%20%28single-precision%29))
  (bind _righteye (Variables|Default|GetRightEye))
  (bind _lefteye (Variables|Default|GetLeftEye))
  (Utilities|FlowControl|Sequence
    (:then_0
      (Pawn|Input|AddMovementInput "0.000000,-1.000000, 0" AxisValue false))
    (:then_1
      (if (>= AxisValue 0.0)
        (if (== AxisValue 0.0)
          (Rendering|SetVisibility (Variables|Default|GetRightEye) false false)
          (Rendering|SetVisibility (Variables|Default|GetLeftEye) false false)
          (Rendering|SetVisibility (Variables|Default|GetMiddleEye) true false)
          (else
            (Rendering|SetVisibility _righteye true false)
            (Rendering|SetVisibility _lefteye false false)
            (Rendering|SetVisibility (Variables|Default|GetMiddleEye) false false)))
        (else
          (Rendering|SetVisibility _righteye false false)
          (Rendering|SetVisibility _lefteye true false)
          (Rendering|SetVisibility (Variables|Default|GetMiddleEye) false false))))))

(fn ConstructionScript)