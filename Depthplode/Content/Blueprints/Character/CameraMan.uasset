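; CameraMan is a camera actor that follows the player vertically and drives level spawning as the player reaches new layers.
; After a short BeginPlay delay, it reads block size and camera Y from Main_GM and becomes the player controller's view target.
; Each Tick it tracks player height at fixed X and Y, calling SpawnBlocks on Main_GM whenever absolute Z, measured in block widths, exceeds the previous maximum.
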(event EventBeginPlay
  (Utilities|FlowControl|Delay 0.1)
  (bind _asmain_gm (Utilities|Casting|CastToMain_GM (Game|GetGameMode)))
  (Variables|Default|SetCube_Width (Variables|/Game/Blueprints/Gamemode/Main_GM.Main_GM_C|GetBox_Size _asmain_gm))
  (Variables|Default|SetMax_Z (Math|Float|Round (/ (Math|Float|Absolute(Float) (.Z (Math|Vector|BreakVector (Transformation|GetActorLocation (Game|GetPlayerCharacter 0))))) (Variables|Default|GetCube_Width))))
  (Variables|Default|SetPos_Y (Variables|/Game/Blueprints/Gamemode/Main_GM.Main_GM_C|GetCamera_Pos_Y _asmain_gm))
  (Game|Player|SetViewTargetwithBlend (Game|GetPlayerController 0) self 0.0 "VTBlend_Linear" 0.0 false))

(event Collision|EventActorBeginOverlap
  (params (OtherActor :type Actor%20Object%20Reference)))

(event EventTick
  (params (DeltaSeconds :type Float%20%28single-precision%29))
  (bind _returnvalue (Game|GetPlayerCharacter 0))
  (bind _cube_width (Variables|Default|GetCube_Width))
  (bind _returnvalue_2 (Transformation|GetActorLocation _returnvalue))
  (bind _z (Math|Vector|BreakVector _returnvalue_2))
  (bind _returnvalue_3 (Math|Float|Absolute(Float) _z))
  (bind _returnvalue_4 (/ _returnvalue_3 _cube_width))
  (bind _returnvalue_5 (Math|Float|Round _returnvalue_4))
  (Utilities|FlowControl|Sequence
    (:then_0
      (Utilities|IsValid _returnvalue
        (:Is%20Valid
          (Transformation|SetActorLocation (Math|Vector|MakeVector 2e+03 (Variables|Default|GetPos_Y) (+ _z 5e+02)) false false))))
    (:then_1
      (Utilities|IsValid _returnvalue
        (:Is%20Valid
          (if (> _returnvalue_5 (Variables|Default|GetMax_Z))
            (Variables|Default|SetMax_Z _returnvalue_5)
            (bind _asmain_gm (Utilities|Casting|CastToMain_GM (Game|GetGameMode)))
            (Default|SpawnBlocks _asmain_gm (Variables|/Game/Blueprints/Gamemode/Main_GM.Main_GM_C|GetCurrent_Max_Layer _asmain_gm))))))))

(fn ConstructionScript)