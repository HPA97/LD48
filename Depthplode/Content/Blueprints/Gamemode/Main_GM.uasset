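; Game mode that builds a grid world of cubes stacked downward in layers between two side walls.
; BeginPlay sets world range and camera Y, pre-spawns a hidden pool of randomly textured cubes, generates the starting layers, then positions the walls from world width.
; Each layer uses a random seed in a modulo formula to leave gaps, filling other cells from the pool, a ring buffer that recycles the oldest cubes when exhausted.
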(event Custom|Add_World_References
  (params (Left_Wall :type Static%20Mesh%20Actor%20Object%20Reference) (Right_Wall :type Static%20Mesh%20Actor%20Object%20Reference))
  (Variables|Default|SetLeft_Wall Left_Wall)
  (Variables|Default|SetRight_Wall Right_Wall))

(event Custom|Spawn_Blocks
  (params (Layer :type Integer))
  (Variables|Default|SetRNG (Math|Random|RandomInteger 1000))
  (Math|Integer|IncrementInt (Variables|Default|GetCurrent_Max_Layer)
    (:%20%20
      (for _index (range 0 (- (Math|Float|Truncate (* (Variables|Default|GetWorld_Width) 1.0)) 1))
        (if (not (== (Math|Integer|%(Integer) (+ (+ _index (/ _index (Variables|Default|GetWorld_Width))) (* _index (Math|Integer|%(Integer) (+ (* (Variables|Default|GetRNG) (+ _index (/ _index (Variables|Default|GetWorld_Width)))) (/ _index (Variables|Default|GetWorld_Width))) 83))) 3) 2))
          (bind _cube (CallFunction|GetfromCubeBank))
          (Transformation|SetActorLocation _cube (Math|Vector|MakeVector (.X (Math|Vector|BreakVector (Variables|Default|GetStart_Generate_Position))) (* (Math|Integer|%(Integer) _index (Variables|Default|GetWorld_Width)) (Variables|Default|GetBox_Size)) (* (+ (* Layer (Variables|Default|GetBox_Size)) (* (/ _index (Variables|Default|GetWorld_Width)) (Variables|Default|GetBox_Size))) -1.0)) false false))))))

(event Custom|Set_Wall_Location
  (bind _start_generate_position (Variables|Default|GetStart_Generate_Position))
  (bind (_x _y _z) (Math|Vector|BreakVector _start_generate_position))
  (Utilities|FlowControl|Sequence
    (:then_0
      (Transformation|SetActorLocation (Variables|Default|GetLeft_Wall) (Math|Vector|MakeVector _x (+ (* (+ (Variables|Default|GetWorld_Width) 1) (Variables|Default|GetBox_Size)) (Variables|Default|GetWall_Offset_Left)) _z) false false))
    (:then_1
      (Transformation|SetActorLocation (Variables|Default|GetRight_Wall) (Math|Vector|MakeVector _x (Variables|Default|GetWall_Offset_Right) _z) false false))))

(event Custom|Update_Camera_Pos_Y
  (Variables|Default|SetCamera_Pos_Y (* (/ (Variables|Default|GetWorld_Width) 2) (Variables|Default|GetBox_Size))))

(event Custom|Update_World_Range
  (Variables|Default|SetWorld_Range (* (Variables|Default|GetWorld_Width) (Variables|Default|GetBox_Size))))

(event Custom|Create_Cubes
  (for _index (range 0 (- (* (Variables|Default|GetWorld_Width) 30) 1))
    (bind _returnvalue (Game|SpawnActorfromClass "/Game/Objects/Cube.Cube_C" (Math|Transform|MakeTransform (Variables|Default|GetCube_Bank_Location)) "Undefined" 0 0))
    (Utilities|Map|Add (Variables|Default|GetCube_Map) _index _returnvalue)
    (Rendering|SetActorHiddenInGame _returnvalue true)
    (Default|UpdateMaterial _returnvalue (Math|Random|RandomInteger 256))))

(event EventBeginPlay
  (CallFunction|UpdateCameraPosY)
  (CallFunction|UpdateWorldRange)
  (Utilities|FlowControl|Delay 0.1)
  (Utilities|FlowControl|Sequence
    (:then_0
      (CallFunction|CreateCubes))
    (:then_1
      (for _index (range 0 18)
        (CallFunction|SpawnBlocks _index)))
    (:then_2
      (Utilities|FlowControl|Delay 0.4)
      (CallFunction|SetWallLocation))))

(event EventTick
  (params (DeltaSeconds :type Float%20%28single-precision%29)))

(fn ConstructionScript)

(fn GetfromCubeBank
  (if (>= (Variables|Default|GetCube_Bank_Head) (Utilities|Map|Length (Variables|Default|GetCube_Map)))
    (Variables|Default|SetCube_Bank_Head 0))
  (LocalVariables|SetReturn_Cube (.Value (Utilities|Map|Find (Variables|Default|GetCube_Map) (Variables|Default|GetCube_Bank_Head))))
  (Math|Integer|IncrementInt (Variables|Default|GetCube_Bank_Head)
    (:%20%20
      (Rendering|SetActorHiddenInGame (LocalVariables|GetReturn_Cube) false)
      (return (LocalVariables|GetReturn_Cube)))))